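; BP_BlockRotatingTest is a prototype level prop that continuously rotates and visualizes its change in facing.
; Tick runs ServerRotateFloor only with authority, adding world rotation from the RollPitchYaw rates scaled by delta time.
; BeginPlay stores and draws the initial forward vector as a long-lived debug arrow.
; Each rotation step draws the current forward arrow and prints the dot product of both vectors, each scaled by 100.
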(event Custom|ServerRotateFloor
  (params (Delta :type Float%20%28double-precision%29))
  (bind _returnvalue (Transformation|GetActorLocation))
  (bind _returnvalue_2 (Transformation|GetActorForwardVector))
  (bind _rollpitchyaw (Variables|Default|GetRollPitchYaw))
  (bind _returnvalue_3 (* _returnvalue_2 "100.000000,100.000000,100.000000"))
  ;[1 1 1] Server rotate shape
  (Class|Actor|AddActorWorldRotation (Math|Rotator|MakeRotator (* Delta (.x _rollpitchyaw)) (* Delta (.y _rollpitchyaw)) (* Delta (.z _rollpitchyaw))))
  (Rendering|Debug|DrawDebugArrow _returnvalue (+ _returnvalue _returnvalue_3) 0.0 "(R=0.145961,G=0.000000,B=1.000000,A=1.000000)" 0.0 2.0)
  (Development|PrintText (Utilities|Text|ToText(Float) (Math|Vector|DotProduct (* (stale EventBeginPlay _output_get) "100.000000,100.000000,100.000000") _returnvalue_3) "HalfToEven")))

(event EventBeginPlay
  (bind _returnvalue (Transformation|GetActorLocation))
  (bind _output_get (Variables|Default|SetInitialForward (Transformation|GetActorForwardVector)))
  (Rendering|Debug|DrawDebugArrow _returnvalue (+ _returnvalue (* _output_get "100.000000,100.000000,100.000000")) 0.0 "(R=1.000000,G=0.000000,B=0.030531,A=1.000000)" 999.0 2.0))

(event Collision|EventActorBeginOverlap
  (params (OtherActor :type Actor%20Object%20Reference)))

(event EventTick
  (params (DeltaSeconds :type Float%20%28single-precision%29))
  (Networking|SwitchHasAuthority
    (:Authority
      (CallFunction|ServerRotateFloor DeltaSeconds))))

(fn ConstructionScript)