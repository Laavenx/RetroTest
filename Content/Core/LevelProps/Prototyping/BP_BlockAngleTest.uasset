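; BP_BlockAngleTest is a prototype actor for visualizing vector rotation around an axis.
; Each tick it draws a thin red debug arrow along its forward vector from its location.
; It also draws a thicker cyan arrow showing that vector rotated by the Angle variable around the Axis variable, so the resulting direction can be compared.
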(event EventBeginPlay)

(event EventTick
  (params (DeltaSeconds :type Float%20%28single-precision%29))
  (bind _returnvalue (Transformation|GetActorLocation))
  (bind _returnvalue_2 (Transformation|GetActorForwardVector))
  (Rendering|Debug|DrawDebugArrow _returnvalue (+ _returnvalue (Math|Vector|RotateVectorAroundAxis (* _returnvalue_2 "100.000000,100.000000,100.000000") (Variables|Default|GetAngle) (Variables|Default|GetAxis))) 2.0 "(R=0.000000,G=0.945939,B=1.000000,A=1.000000)" 0.0 4.0)
  (Rendering|Debug|DrawDebugArrow _returnvalue (+ _returnvalue (* _returnvalue_2 "100.000000,100.000000,100.000000")) 2.0 "(R=1.000000,G=0.000000,B=0.059706,A=1.000000)" 0.0 1.0))

(fn ConstructionScript)