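; Moving block level prop that shuttles its cube back and forth between its local origin and LocationEnd.
; On BeginPlay only the authority starts ServerMove, whose timeline adds unswept local offsets along the normalized end vector each update.
; When the timeline finishes, DidReachEndLocation compares the cube's relative location per axis, flips MoveBack if the limit is reached, then ServerMove restarts.
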(event Custom|ServerMove
  (bind _shape_cube (Variables|Default|GetShape_Cube))
  ;[1 1 1] Server Replicated Rotation
  (bind _locationoffset (Timeline|Timeline PlayFromStart)
    (:Update
      (if (Variables|Default|GetbMoveBack)
        (Transformation|AddLocalOffset _shape_cube (* (* _locationoffset (Math|Vector|Normalize (Variables|Default|GetLocationEnd))) "-1.000000,-1.000000,-1.000000") false false)
        (else
          (Transformation|AddLocalOffset _shape_cube (* _locationoffset (Math|Vector|Normalize (Variables|Default|GetLocationEnd))) false false))))
    (:Finished
      (bind _didreach (CallFunction|DidReachEndLocation))
      (if _didreach
        (Variables|Default|SetbMoveBack (not (Variables|Default|GetbMoveBack))))
      (CallFunction|ServerMove))))

(event EventBeginPlay
  (Networking|SwitchHasAuthority
    (:Authority
      (CallFunction|ServerMove))))

(event Collision|EventActorBeginOverlap
  (params (OtherActor :type Actor%20Object%20Reference)))

(event EventTick
  (params (DeltaSeconds :type Float%20%28single-precision%29)))

(fn ConstructionScript)

(fn DidReachEndLocation
  (bind (_x _y _z) (Math|Vector|BreakVector "0, 0, 0"))
  (bind _shape_cube (Variables|Default|GetShape_Cube))
  (bind _locationend (Variables|Default|GetLocationEnd))
  (bind _shape_cube_2 (Variables|Default|GetShape_Cube))
  (bind _locationend_2 (Variables|Default|GetLocationEnd))
  (bind _returnvalue (Math|Vector|VectorGetAbs _locationend_2))
  (bind _returnvalue_2 (Math|Vector|Normalize _locationend))
  (bind _relativelocation (Variables|/Script/Engine.SceneComponent|GetRelativeLocation _shape_cube))
  (bind _relativelocation_2 (Variables|/Script/Engine.SceneComponent|GetRelativeLocation _shape_cube_2))
  (bind (_x_2 _y_2 _z_2) (Math|Vector|BreakVector _returnvalue))
  (bind _returnvalue_3 (Math|Vector|VectorGetAbs _relativelocation_2))
  (bind _returnvalue_4 (* _returnvalue_2 _relativelocation))
  (bind (_x_3 _y_3 _z_3) (Math|Vector|BreakVector _returnvalue_4))
  (bind (_x_4 _y_4 _z_4) (Math|Vector|BreakVector _returnvalue_3))
  (if (Variables|Default|GetbMoveBack)
    (return (Math|Boolean|ANDBoolean (<= _x_3 _x) (<= _y_3 _y) (<= _z_3 _z)))
    (else
      (return (Math|Boolean|ANDBoolean (>= _x_4 _x_2) (>= _y_4 _y_2) (>= _z_4 _z_2))))))