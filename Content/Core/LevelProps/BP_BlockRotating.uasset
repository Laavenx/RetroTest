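; BP_BlockRotating is a level prop block that rotates its ShapeCube endlessly in steps.
; On BeginPlay, only the authority calls ServerRotateFloor, which seeds CurrentRotation from Transform's X-vector rotation plus RotateBy.
; It then loops latent MoveComponentTo calls, each lasting MovementTime on the shortest path, adding RotateBy through the AddRotators helper after every step.
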(event Custom|ServerRotateFloor
  ;[1 1 1] Server Replicated Rotation
  (bind _outrotator (CallFunction|AddRotators (Math|Conversions|RotationFromXVector (Variables|Default|GetTransform)) (Variables|Default|GetRotateBy)))
  (bind _output_get (Variables|Default|SetCurrentRotation _outrotator))
  (Components|MoveComponentTo (Variables|Default|GetShape_Cube) "0, 0, 0" _output_get false false (Variables|Default|GetMovementTime) true :!label _label)
  (bind _outrotator_2 (CallFunction|AddRotators (Variables|Default|GetCurrentRotation) (Variables|Default|GetRotateBy)))
  (bind _output_get_2 (Variables|Default|SetCurrentRotation _outrotator_2))
  (Components|MoveComponentTo (Variables|Default|GetShape_Cube) "0, 0, 0" _output_get_2 false false (Variables|Default|GetMovementTime) true)
  (bind _outrotator_3 (CallFunction|AddRotators (Variables|Default|GetCurrentRotation) (Variables|Default|GetRotateBy)))
  (Variables|Default|SetCurrentRotation _outrotator_3)
  (goto _label))

(event Collision|EventActorBeginOverlap
  (params (OtherActor :type Actor%20Object%20Reference)))

(event EventBeginPlay
  (Networking|SwitchHasAuthority
    (:Authority
      (CallFunction|ServerRotateFloor))))

(fn ConstructionScript)

(fn AddRotators
  (params (RotatorA :type Rotator) (RotatorB :type Rotator))
  (return (Math|Rotator|CombineRotators RotatorA RotatorB)))